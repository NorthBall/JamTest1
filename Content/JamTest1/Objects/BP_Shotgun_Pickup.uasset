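; Shotgun pickup actor that grants the player character a timed shotgun weapon when they enter its pickup box.
; On entry it records whether the shotgun effect tag is already present, then applies that tag for a fixed duration.
; If application succeeds, it adds the weapon and prints a debug message only for characters lacking the effect, then destroys itself either way.
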(event `self.OnEnterPickupBox`
  (params (OverlappedComp :type "PrimitiveComponent Object Reference") (Other :type "Actor Object Reference") (OtherComp :type "PrimitiveComponent Object Reference") (OtherBodyIndex :type Integer) (bFromSweep :type Boolean) (SweepResult :type "HitResult Structure (by ref)"))
  (bind _asjam_test_1character (cast `JamTest1Character` Other))
  (bind _returnvalue (`JT_UtilityFunctions.HasEffect` _asjam_test_1character (struct :`TagName` "Effect.Weapon.Shotgun")))
  (bind _returnvalue_2 (`JT_UtilityFunctions.ApplyEffect` _asjam_test_1character (struct :`TagName` "Effect.Weapon.Shotgun") 30.0))
  (if _returnvalue_2
    (`|ExecutionSequence`
      (:`then_0`
        (if (not _returnvalue)
          (`JamTest1Character.AddWeapon` _asjam_test_1character (struct :`TagName` "Effect.Weapon.Shotgun"))
          (`KismetSystemLibrary.PrintString` "Shotgun")))
      (:`then_1`
        (`self.K2_DestroyActor`)))))

(fn `UserConstructionScript`
  (`parent.UserConstructionScript`))