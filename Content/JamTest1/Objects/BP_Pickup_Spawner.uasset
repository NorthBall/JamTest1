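; BP_Pickup_Spawner is an actor that spawns a random pickup at its own transform and replenishes it once it is gone.
; BeginPlay delays the first spawn by a short random time.
; SpawnPickupIfNeeded spawns a class drawn from the Classes array when the stored Pickup is invalid, then starts a looping timer on itself to periodically recheck.
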(event `SpawnPickupIfNeeded`
  (if (not (`KismetSystemLibrary.IsValid` (`self.Pickup`)))
    (bind _returnvalue (`|SpawnActorFromClass` (`KismetArrayLibrary.Array_Random` (`self.Classes`)) (`self.GetTransform`) "Undefined" "MultiplyWithRoot" null null))
    (set `self.Pickup` _returnvalue)
    (`KismetSystemLibrary.K2_SetTimer` null "SpawnPickupIfNeeded" 20.0 true)))

(event `self.ReceiveBeginPlay`
  (`KismetSystemLibrary.K2_SetTimer` null "SpawnPickupIfNeeded" (`KismetMathLibrary.RandomFloatInRange` 0.0 5.0)))

(fn `UserConstructionScript`)