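; Melee zombie enemy Blueprint that chases and punches the player.
; Shortly after BeginPlay it finds the JamTest1Character and uses AIMoveTo to close to attack range.
; On arrival it plays a punch montage, waits a pre-attack delay, then plays a sound and deals damage without rechecking range.
; It then resumes the chase, looping while the target stays valid.
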(event `self.ReceiveBeginPlay`
  (`KismetSystemLibrary.Delay` 2.0)
  (`self.FindPlayer`))

(event `FindPlayer`
  (bind _returnvalue (`GameplayStatics.GetActorOfClass` "/Script/JamTest1.JamTest1Character"))
  (`/Engine/EditorBlueprintResources/StandardMacros.IsValid` _returnvalue
    (:`Is Valid`
      (set `self.TargetedPlayer` _returnvalue)
      (`self.ContinueMove`))))

(event `self.TargetPlayer`
  (params (Player :type "Actor Object Reference"))
  (set `self.TargetedPlayer` Player)
  (`self.ContinueMove`))

(event `ContinueMove`
  (`|AIMoveTo` self (0.0 0.0 10.0) (`self.TargetedPlayer`) (`self.AttackRange_0`)
    (:`OnSuccess`
      (`self.OnTargetInRange`))))

(event `OnTargetInRange`
  (`|PlayMontage` (`self.SkeletalMesh`) "/Game/JamTest1/Enemies/Animations/ZombiePunching_UE_Montage.ZombiePunching_UE_Montage"
    (:`then`
      (`KismetSystemLibrary.Delay` (`self.PreAttackDelay`))
      (`self.PerformAttack`))))

(event `PerformAttack`
  (bind _targetedplayer (`self.TargetedPlayer`))
  (`|ExecutionSequence`
    (:`then_0`
      (`/Engine/EditorBlueprintResources/StandardMacros.IsValid` _targetedplayer
        (:`Is Valid`
          (`GameplayStatics.PlaySound2D` "/Game/JamTest1/Sounds/zombie_attack.zombie_attack" 1.0 1.0 0.0 null null)
          (`JT_UtilityFunctions.DealDamage` _targetedplayer self (`self.AttackDamage`)))))
    (:`then_1`
      (`/Engine/EditorBlueprintResources/StandardMacros.IsValid` (`self.TargetedPlayer`)
        (:`Is Valid`
          (`self.ContinueMove`))))))

(fn `UserConstructionScript`)