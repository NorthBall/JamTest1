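; BP_EnemySpawner is an enemy zone controller that sends the enemies inside its BoxOfControl volume after the player; despite its name, it spawns nothing.
; Overlap events add JT_Enemy actors to ControlledEnemies and remove them when they leave.
; A player entering calls TargetPlayer on each valid tracked enemy, with debug prints.
; A delayed BeginPlay scan registers enemies, then players, already inside the box.
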(event `self.ReceiveBeginPlay`
  (`KismetSystemLibrary.Delay` 1.0)
  (for _array_element (`PrimitiveComponent.GetOverlappingActors` (`self.BoxOfControl`) "/Script/JamTest1.JT_Enemy")
    (`self.OnEnemyCollide` _array_element))
  (for _array_element_2 (`PrimitiveComponent.GetOverlappingActors` (`self.BoxOfControl`) "/Script/JamTest1.JamTest1Character")
    (`self.OnPlayerCollide` _array_element_2)))

(event `self.BoxOfControl.OnComponentBeginOverlap`
  (params (OverlappedComponent :type "PrimitiveComponent Object Reference") (OtherActor :type "Actor Object Reference") (OtherComp :type "PrimitiveComponent Object Reference") (OtherBodyIndex :type Integer) (bFromSweep :type Boolean) (SweepResult :type "HitResult Structure (by ref)"))
  (bind _returnvalue (`GameplayStatics.GetObjectClass` OtherActor))
  (if (`KismetMathLibrary.ClassIsChildOf` _returnvalue "/Script/JamTest1.JamTest1Character")
    (`self.OnPlayerCollide` OtherActor)
    (elif (`KismetMathLibrary.ClassIsChildOf` _returnvalue "/Script/JamTest1.JT_Enemy")
      (`self.OnEnemyCollide` OtherActor))))

(event `self.BoxOfControl.OnComponentEndOverlap`
  (params (OverlappedComponent :type "PrimitiveComponent Object Reference") (OtherActor :type "Actor Object Reference") (OtherComp :type "PrimitiveComponent Object Reference") (OtherBodyIndex :type Integer))
  (if (`KismetMathLibrary.ClassIsChildOf` (`GameplayStatics.GetObjectClass` OtherActor) "/Script/JamTest1.JT_Enemy")
    (`self.OnEnemyOutOfControl` OtherActor)))

(fn `OnEnemyCollide`
  (params (Actor :type "Actor Object Reference"))
  (`/Engine/EditorBlueprintResources/StandardMacros.IsValid` Actor
    (:`Is Valid`
      (bind _asjt_enemy (cast `JT_Enemy` Actor))
      (`KismetArrayLibrary.Array_AddUnique` (`self.ControlledEnemies`) _asjt_enemy))))

(fn `OnEnemyOutOfControl`
  (params (Actor :type "Actor Object Reference"))
  (bind _asjt_enemy (cast `JT_Enemy` Actor))
  (`KismetArrayLibrary.Array_RemoveItem` (`self.ControlledEnemies`) _asjt_enemy))

(fn `OnPlayerCollide`
  (params (Player :type "Actor Object Reference"))
  (for _array_element (`self.ControlledEnemies`)
    (`/Engine/EditorBlueprintResources/StandardMacros.IsValid` _array_element
      (:`Is Valid`
        (`JT_Enemy.TargetPlayer` _array_element Player)
        (`KismetSystemLibrary.PrintString` (`KismetSystemLibrary.GetDisplayName` _array_element) true false (struct :`R` 0.200359 :`B` 1.0 :`A` 1.0) 3.0))
      (:`Is Not Valid`
        (`KismetSystemLibrary.PrintString` "StoreInvalidEnemy" true false (struct :`R` 0.578125 :`B` 0.017688 :`A` 1.0) 10.0)))))

(fn `UserConstructionScript`)