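; BP_Spawner is a phase-driven enemy spawner whose spawn point advances along a spline between phases.
; When a phase flagged to move ends, Tick slides SpawnPoint to the next spline point, then starts the next phase.
; SpawnEnemy places enemies at random reachable locations around SpawnPoint with random yaw, retrying failed spawns up to a fixed limit.
; The per-class height offset is a stub returning zero.
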(event `self.ReceiveTick`
  (params (DeltaSeconds :type "Float (single-precision)"))
  (bind _currentdistance (`self.CurrentDistance`))
  (if (`self.ShouldMove`)
    (bind _distance (`self.GetSectionEnd`))
    (if (> _distance 0.0)
      (`self.MoveInLocalDistance` DeltaSeconds)
      (`self.MoveSpawnPoint` _currentdistance)
      (if (>= _currentdistance _distance)
        (set `self.CurrentDistance` _distance)
        (set `self.ShouldMove` false)
        (set `self.CurrentSplinePoint` (`self.GetNextPoint`))
        (`self.StartNextPhase`)))))

(event `self.SpawnEnemy`
  (params (EnemyClass :type "Object Class Reference") (SpawnRadius :type "Float (single-precision)"))
  (bind _randomlocation (`NavigationSystemV1.K2_GetRandomReachablePointInRadius` (`SceneComponent.K2_GetComponentLocation` (`self.SpawnPoint`)) SpawnRadius null null))
  (bind _asactor (castclass `Actor` EnemyClass))
  (bind _returnvalue (`|SpawnActorFromClass` _asactor (`KismetMathLibrary.MakeTransform` (`KismetMathLibrary.MakeVector` (.x _randomlocation) (.y _randomlocation) (+ (.z _randomlocation) (`self.GetHeightByClass` _asactor))) (`KismetMathLibrary.MakeRotator` 0.0 0.0 (`KismetMathLibrary.RandomFloatInRange` 0.0 360.0))) "AdjustIfPossibleButDontSpawnIfColliding" "MultiplyWithRoot" null null))
  (`/Engine/EditorBlueprintResources/StandardMacros.IsValid` _returnvalue
    (:`Is Valid`
      (set `self.FailedToSpawn` 0))
    (:`Is Not Valid`
      (bind _result (`/Engine/EditorBlueprintResources/StandardMacros.IncrementInt` (`self.FailedToSpawn`))
        (:`  `
          (if (< _result 10)
            (`self.SpawnEnemy` _asactor SpawnRadius)
            (else
              (set `self.FailedToSpawn` 0))))))))

(event `self.OnPhaseEnded`
  (params (Phase :type "JT_SpawnerPhase Structure"))
  (`parent.OnPhaseEnded` Phase)
  (if (`.MoveOnPhaseEnded` (break `JT_SpawnerPhase` Phase))
    (set `self.ShouldMove` true)))

(fn `GetHeightByClass`
  (params (Class :type "Actor Class Reference"))
  (returns (Height :type "Float (double-precision)"))
  (return 0.0))

(fn `GetNextPoint`
  (returns (Index :type Integer))
  (return (+ (`self.CurrentSplinePoint`) 1)))

(fn `GetSectionEnd`
  (returns (Distance :type "Float (double-precision)"))
  (bind _index (`self.GetNextPoint`))
  (bind _spline (`self.Spline`))
  (if (>= (`SplineComponent.GetNumberOfSplinePoints` _spline) _index)
    (return (`SplineComponent.GetDistanceAlongSplineAtSplinePoint` _spline _index))
    (else
      (return 0.0))))

(fn `MoveInLocalDistance`
  (params (DeltaTime :type "Float (double-precision)"))
  (set `self.CurrentDistance` (+ (`self.CurrentDistance`) (* DeltaTime (`self.SplineSpeed`)))))

(fn `MoveSpawnPoint`
  (params (SplineDistance :type "Float (double-precision)"))
  (`SceneComponent.K2_SetRelativeLocation` (`self.SpawnPoint`) (`SplineComponent.GetLocationAtDistanceAlongSpline` (`self.Spline`) SplineDistance "Local") false false))

(fn `UserConstructionScript`)