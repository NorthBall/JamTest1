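; BP_EnemyFarm_Melee is a melee enemy that seeks out and attacks neutral entities, treated as plants.
; Two seconds after spawning, it targets the first JT_NeutralEntity found and walks to it with AIMoveTo.
; In range, it plays a punch montage, then deals damage after a delay, looping until the target is invalid and searching again.
; TargetPlayer stores a player reference that this graph never uses.
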(event `self.ReceiveBeginPlay`
  (`KismetSystemLibrary.Delay` 2.0)
  (`self.FindPlant`))

(event `FindPlant`
  (bind _returnvalue (`GameplayStatics.GetActorOfClass` "/Script/JamTest1.JT_NeutralEntity"))
  (`/Engine/EditorBlueprintResources/StandardMacros.IsValid` _returnvalue
    (:`Is Valid`
      (set `self.TargetedPlant` _returnvalue)
      (`self.ContinueMove`))))

(event `self.TargetPlayer`
  (params (Player :type "Actor Object Reference"))
  (set `self.TargetedPlayer_0` Player))

(event `ContinueMove`
  (`|AIMoveTo` self (0.0 0.0 0.0) (`self.TargetedPlant`) (`self.AttackRange_0`) true
    (:`OnSuccess`
      (`self.OnTargetInRange`))
    (:`OnFail`
      (`self.FindPlant`))))

(event `OnTargetInRange`
  (`KismetSystemLibrary.PrintString` "Hello")
  (`|PlayMontage` (`self.SkeletalMesh`) "/Game/JamTest1/Enemies/Animations/ZombiePunching_UE_Montage.ZombiePunching_UE_Montage"
    (:`then`
      (`KismetSystemLibrary.Delay` (`self.PreAttackDelay_0`))
      (`self.PerformAttack`))))

(event `PerformAttack`
  (bind _targetedplant (`self.TargetedPlant`))
  (`|ExecutionSequence`
    (:`then_0`
      (`/Engine/EditorBlueprintResources/StandardMacros.IsValid` _targetedplant
        (:`Is Valid`
          (`GameplayStatics.PlaySoundAtLocation` "/Game/JamTest1/Sounds/zombie_attack.zombie_attack" (`self.K2_GetActorLocation`) (struct) 1.0 1.0 0.0 null null null null)
          (`JT_UtilityFunctions.DealDamage` _targetedplant self (`self.AttackDamage`)))))
    (:`then_1`
      (`/Engine/EditorBlueprintResources/StandardMacros.IsValid` (`self.TargetedPlant`)
        (:`Is Valid`
          (`self.ContinueMove`))
        (:`Is Not Valid`
          (`self.FindPlant`))))))

(fn `UserConstructionScript`)