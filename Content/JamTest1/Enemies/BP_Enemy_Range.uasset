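; Ranged enemy that chases a targeted player and fires projectiles once within attack range.
; TargetPlayer stores the target and starts an AI MoveTo, using AttackRange as the acceptance radius.
; On arrival it waits PreAttackDelay, turns to face the target and spawns BP_Enemy_Range_Projectile along its yaw, then moves again.
; The cycle is event-driven without Tick, repeats only on successful moves, and fires without rechecking range after the delay.
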(event `self.TargetPlayer`
  (params (Player :type "Actor Object Reference"))
  (set `self.TargetedPlayer` Player)
  (`self.ContinueMove`))

(event `ContinueMove`
  (`|AIMoveTo` self (0.0 0.0 10.0) (`self.TargetedPlayer`) (`self.Attack Range`)
    (:`OnSuccess`
      (`self.OnPlayerInRange`))))

(event `OnPlayerInRange`
  (`KismetSystemLibrary.Delay` (`self.PreAttackDelay`))
  (`self.PerformAttack`)
  (`self.ContinueMove`))

(event `PerformAttack`
  (bind (_returnvalue_roll _returnvalue_pitch _returnvalue_yaw) (`KismetMathLibrary.BreakRotator` (`self.K2_GetActorRotation`)))
  (`self.K2_SetActorRotation` (`KismetMathLibrary.FindLookAtRotation` (`self.K2_GetActorLocation`) (`self.K2_GetActorLocation` (`self.TargetedPlayer`))))
  (`|SpawnActorFromClass` "/Game/JamTest1/Enemies/BP_Enemy_Range_Projectile.BP_Enemy_Range_Projectile_C" (`KismetMathLibrary.MakeTransform` (`self.K2_GetActorLocation`) (`KismetMathLibrary.MakeRotator` 0.0 0.0 _returnvalue_yaw)) "AlwaysSpawn" "MultiplyWithRoot" self null))

(fn `UserConstructionScript`)