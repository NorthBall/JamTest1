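; Melee enemy Blueprint that chases a targeted player and punches them.
; TargetPlayer stores the player and starts an AI MoveTo that, on reaching attack range, waits a pre-attack delay, attacks, then immediately resumes the chase.
; The attack plays a zombie punch montage whose notify deals fixed damage to the target, with no range recheck.
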(event `self.TargetPlayer`
  (params (Player :type "Actor Object Reference"))
  (set `self.TargetedPlayer` Player)
  (`self.ContinueMove`))

(event `ContinueMove`
  (`|AIMoveTo` self (0.0 0.0 10.0) (`self.TargetedPlayer`) (`self.AttackRange`)
    (:`OnSuccess`
      (`self.OnPlayerInRange`))))

(event `OnPlayerInRange`
  (`KismetSystemLibrary.Delay` (`self.PreAttackDelay`))
  (`self.PerformAttack`)
  (`self.ContinueMove`))

(event `PerformAttack`
  (`|PlayMontage` null "/Game/JamTest1/Enemies/Animations/ZombiePunching_UE_Montage.ZombiePunching_UE_Montage"
    (:`OnNotifyBegin`
      (`JT_UtilityFunctions.DealDamage` (`self.TargetedPlayer`) null 5.0))))

(fn `UserConstructionScript`)