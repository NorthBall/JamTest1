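; BP_EnemyPlayer_UFO is a UFO enemy Blueprint that acquires the player character as its target.
; Shortly after BeginPlay, FindPlayer looks up the JamTest1Character actor, stores it as TargetedPlayer and calls ContinueMove.
; The movement logic behind ContinueMove is not defined in these graphs, and the lookup does not retry if no character is found.
; Overlap and Tick events are disabled stubs, and the construction script only calls its parent.
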(event `self.ReceiveBeginPlay`
  (`KismetSystemLibrary.Delay` 0.4)
  (`self.FindPlayer`))

(event `FindPlayer`
  (bind _returnvalue (`GameplayStatics.GetActorOfClass` "/Script/JamTest1.JamTest1Character"))
  (`/Engine/EditorBlueprintResources/StandardMacros.IsValid` _returnvalue
    (:`Is Valid`
      (set `self.TargetedPlayer` _returnvalue)
      (`self.ContinueMove`))))

(fn `UserConstructionScript`
  (`parent.UserConstructionScript`))