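; BP_Enemy_UFO is a ranged enemy UFO that chases a player and fires laser projectiles.
; Once given a target, it uses AIMoveTo to get within attack range, pauses, turns to face the player, fires from its projectile point, then resumes moving in a loop.
; Each tick its eye yaws toward the target, or sweeps in randomly chosen directions at timed intervals when no valid target exists.
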(event `UpdateEyeLook`
  (params (DeltaTime :type "Float (double-precision)"))
  (bind _targetedplayer (`self.TargetedPlayer`))
  (bind _eye (`self.Eye`))
  (bind (_returnvalue_roll _returnvalue_pitch _returnvalue_yaw) (`KismetMathLibrary.BreakRotator` (`KismetMathLibrary.FindLookAtRotation` (`SceneComponent.K2_GetComponentLocation` _eye) (`self.K2_GetActorLocation` _targetedplayer))))
  (`/Engine/EditorBlueprintResources/StandardMacros.IsValid` _targetedplayer
    (:`Is Valid`
      (`SceneComponent.K2_SetWorldRotation` _eye (`KismetMathLibrary.MakeRotator` 0.0 0.0 _returnvalue_yaw) false false))
    (:`Is Not Valid`
      (`self.RandomEyeMovement` DeltaTime))))

(event `self.ReceiveTick`
  (params (DeltaSeconds :type "Float (single-precision)"))
  (`self.UpdateEyeLook` DeltaSeconds))

(event `self.TargetPlayer`
  (params (Player :type "Actor Object Reference"))
  (set `self.TargetedPlayer` Player)
  (`self.ContinueMove`))

(event `ContinueMove`
  (`|AIMoveTo` self (0.0 0.0 10.0) (`self.TargetedPlayer`) (`self.Attack Range`)
    (:`OnSuccess`
      (`self.OnPlayerInRange`))))

(event `OnPlayerInRange`
  (`KismetSystemLibrary.Delay` (`self.PreAttackDelay`))
  (`self.PerformAttack`)
  (`self.ContinueMove`))

(event `PerformAttack`
  (`self.K2_SetActorRotation` (`KismetMathLibrary.FindLookAtRotation` (`self.K2_GetActorLocation`) (`self.K2_GetActorLocation` (`self.TargetedPlayer`))))
  (`GameplayStatics.PlaySound2D` "/Game/JamTest1/Sounds/lazer_fire.lazer_fire" 1.0 1.0 0.0 null null)
  (`JT_UtilityFunctions.SpawnProjectile` self "/Game/JamTest1/Enemies/BP_Enemy_Range_Projectile.BP_Enemy_Range_Projectile_C" (`self.ProjectilePoint`)))

(fn `RandomEyeMovement`
  (params (DeltaTime :type "Float (double-precision)"))
  (locals (EyeLoopDuration :type "Float (double-precision)" :default 2.0) (EyeLoopAngle :type "Float (double-precision)" :default 100.0))
  (bind _eye (`self.Eye`))
  (bind (_returnvalue_roll _returnvalue_pitch _returnvalue_yaw) (`KismetMathLibrary.BreakRotator` (`SceneComponent.K2_GetComponentRotation` _eye)))
  (`|ExecutionSequence`
    (:`then_0`
      (`SceneComponent.K2_SetWorldRotation` _eye (`KismetMathLibrary.MakeRotator` 0.0 0.0 (+ _returnvalue_yaw (* (/ DeltaTime (`local.EyeLoopDuration`)) (`local.EyeLoopAngle`) (`self.EyeDirection`)))) false false))
    (:`then_1`
      (bind _output_get (set `self.EyeTime` (+ (`self.EyeTime`) DeltaTime)))
      (if (> _output_get (`local.EyeLoopDuration`))
        (set `self.EyeDirection` (`KismetMathLibrary.SelectInt` -1 1 (`KismetMathLibrary.RandomBool`)))
        (set `self.EyeTime` 0.0)))))

(fn `UserConstructionScript`)