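; BP_EnemyFarm_Melee1 is a melee farm enemy that hunts and attacks plants (JT_NeutralEntity actors).
; After a spawn delay it grabs the first plant found and walks into attack range with AIMoveTo.
; It plays a punch montage, deals damage after a wind-up delay, then repeats, finding another plant if the target is invalid.
; TargetPlayer stores a player reference, which this graph never uses.
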(event `self.ReceiveBeginPlay`
  (`KismetSystemLibrary.Delay` 2.0)
  (`self.FindPlant`))

(event `FindPlant`
  (bind _returnvalue (`GameplayStatics.GetActorOfClass` "/Script/JamTest1.JT_NeutralEntity"))
  (`/Engine/EditorBlueprintResources/StandardMacros.IsValid` _returnvalue
    (:`Is Valid`
      (set `self.TargetedPlant` _returnvalue)
      (`self.ContinueMove`))))

(event `self.TargetPlayer`
  (params (Player :type "Actor Object Reference"))
  (set `self.TargetedPlayer` Player))

(event `ContinueMove`
  (`|AIMoveTo` self (0.0 0.0 10.0) (`self.TargetedPlant`) (`self.AttackRange`)
    (:`OnSuccess`
      (`self.OnTargetInRange`))))

(event `OnTargetInRange`
  (`|PlayMontage` (`self.SkeletalMesh`) "/Game/JamTest1/Enemies/Animations/ZombiePunching_UE_Montage.ZombiePunching_UE_Montage"
    (:`then`
      (`KismetSystemLibrary.Delay` (`self.PreAttackDelay`))
      (`self.PerformAttack`))))

(event `PerformAttack`
  (bind _targetedplant (`self.TargetedPlant`))
  (`|ExecutionSequence`
    (:`then_0`
      (`/Engine/EditorBlueprintResources/StandardMacros.IsValid` _targetedplant
        (:`Is Valid`
          (`JT_UtilityFunctions.DealDamage` _targetedplant self (`self.AttackDamage`)))))
    (:`then_1`
      (`/Engine/EditorBlueprintResources/StandardMacros.IsValid` (`self.TargetedPlant`)
        (:`Is Valid`
          (`self.ContinueMove`))
        (:`Is Not Valid`
          (`self.FindPlant`))))))

(fn `UserConstructionScript`)