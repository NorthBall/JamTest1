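; UFO farmer enemy that hunts neutral entities, treated as plants, and shoots them with ranged projectiles.
; Shortly after spawning it picks a random JT_NeutralEntity and uses AIMoveTo to close within attack range, picking again if the move fails.
; After a pre-attack delay it faces the target, plays a laser sound and fires.
; It repeats this loop until the target becomes invalid, then picks another.
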(event `self.ReceiveBeginPlay`
  (`KismetSystemLibrary.Delay` 1.0)
  (`self.FindPlant`))

(event `FindPlant`
  (bind _outactors (`GameplayStatics.GetAllActorsOfClass` "/Script/JamTest1.JT_NeutralEntity"))
  (bind _output_get (set `self.TargetedPlant` (`KismetArrayLibrary.Array_Random` _outactors)))
  (`/Engine/EditorBlueprintResources/StandardMacros.IsValid` _output_get
    (:`Is Valid`
      (`self.ContinueMove`))))

(event `self.ContinueMove`
  (`|AIMoveTo` self (0.0 0.0 0.0) (`self.TargetedPlant`) (`self.Attack Range`) true
    (:`OnSuccess`
      (`self.OnPlayerInRange`))
    (:`OnFail`
      (`self.FindPlant`))))

(event `self.PerformAttack`
  (`|ExecutionSequence`
    (:`then_0`
      (`/Engine/EditorBlueprintResources/StandardMacros.IsValid` (`self.TargetedPlant`)
        (:`Is Valid`
          (`self.K2_SetActorRotation` (`KismetMathLibrary.FindLookAtRotation` (`self.K2_GetActorLocation`) (`self.K2_GetActorLocation` (`self.TargetedPlant`))))
          (`GameplayStatics.PlaySound2D` "/Game/JamTest1/Sounds/lazer_fire.lazer_fire" 1.0 1.0 0.0 null null)
          (`JT_UtilityFunctions.SpawnProjectile` self "/Game/JamTest1/Enemies/BP_Enemy_Range_Projectile.BP_Enemy_Range_Projectile_C" (`self.ProjectilePoint`)))))
    (:`then_1`
      (`/Engine/EditorBlueprintResources/StandardMacros.IsValid` (`self.TargetedPlant`)
        (:`Is Valid`
          (`self.ContinueMove`))
        (:`Is Not Valid`
          (`self.FindPlant`))))))

(event `self.OnPlayerInRange`
  (`KismetSystemLibrary.Delay` (`self.PreAttackDelay`))
  (`self.PerformAttack`))

(fn `UserConstructionScript`
  (`parent.UserConstructionScript`))