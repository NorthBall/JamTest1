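; BP_Projectile is a projectile Actor that detects targets through overlap and destroys itself on contact with any actor other than its owner.
; On overlap it calls OnTargetHit if the actor's class derives from TargetedClass, or from JT_NeutralEntity when CanAttackNeutrals is set.
; OnTargetHit is an empty event, leaving the hit effect undefined in this Blueprint.
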(event `self.ReceiveActorBeginOverlap`
  (params (OtherActor :type "Actor Object Reference"))
  (bind _returnvalue (`GameplayStatics.GetObjectClass` OtherActor))
  (if (!= OtherActor (`self.GetOwner`))
    (`|ExecutionSequence`
      (:`then_0`
        (if (`KismetMathLibrary.ClassIsChildOf` _returnvalue (`self.TargetedClass`))
          (`self.OnTargetHit` OtherActor)))
      (:`then_1`
        (if (`self.CanAttackNeutrals`)
          (if (`KismetMathLibrary.ClassIsChildOf` _returnvalue "/Script/JamTest1.JT_NeutralEntity")
            (`self.OnTargetHit` OtherActor))))
      (:`then_2`
        (`self.K2_DestroyActor`)))))

(event `OnTargetHit`
  (params (Target :type "Actor Object Reference")))

(fn `UserConstructionScript`)