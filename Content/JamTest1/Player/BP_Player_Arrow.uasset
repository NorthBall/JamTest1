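; BP_Player_Arrow is the player's arrow, which damages and pushes whatever target it hits.
; Its only active logic is the OnTargetHit event, which calls DealDamage and then AddImpulse on the target with fixed values, passing itself as the source.
; The file contains no movement or hit detection, and its BeginPlay, overlap and Tick events are disabled stubs.
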(event `self.OnTargetHit`
  (params (Target :type "Actor Object Reference"))
  (`JT_UtilityFunctions.DealDamage` Target self 40.0)
  (`JT_UtilityFunctions.AddImpulse` Target self 300.0))

(fn `UserConstructionScript`
  (`parent.UserConstructionScript`))